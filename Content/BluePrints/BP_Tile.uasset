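; BP_Tile is a floor tile actor that counts player characters standing on it and removes itself when crowded.
; Collision overlap begin and end events raise or lower Playercount for BP_ThirdPersonCharacter classes.
; Ten seconds after BeginPlay, a single CheckPlayerCount enables FloorMesh physics and immediately destroys the actor if at least three players are counted.
; It then prints the count as debug text.
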(event `self.ReceiveActorBeginOverlap`
  (params (OtherActor :type "Actor Object Reference")))

(event `self.ReceiveBeginPlay`
  (`KismetSystemLibrary.Delay` 10.0)
  (`self.CheckPlayerCount`)
  (`KismetSystemLibrary.PrintString` (`KismetStringLibrary.Conv_IntToString` (`self.Playercount`)) true true (struct :`R` 0.956597 :`G` 0.830282 :`A` 1.0) 5.0))

(event `self. Collision.OnComponentBeginOverlap`
  (params (OverlappedComponent :type "PrimitiveComponent Object Reference") (OtherActor :type "Actor Object Reference") (OtherComp :type "PrimitiveComponent Object Reference") (OtherBodyIndex :type Integer) (bFromSweep :type Boolean) (SweepResult :type "HitResult Structure (by ref)"))
  (castclass `/Game/ThirdPerson/Blueprints/BP_ThirdPersonCharacter` (`GameplayStatics.GetObjectClass` OtherActor))
  (if true
    (`/Engine/EditorBlueprintResources/StandardMacros.IncrementInt` (`self.Playercount`))))

(event `self. Collision.OnComponentEndOverlap`
  (params (OverlappedComponent :type "PrimitiveComponent Object Reference") (OtherActor :type "Actor Object Reference") (OtherComp :type "PrimitiveComponent Object Reference") (OtherBodyIndex :type Integer))
  (castclass `/Game/ThirdPerson/Blueprints/BP_ThirdPersonCharacter` (`GameplayStatics.GetObjectClass` OtherActor))
  (if true
    (`/Engine/EditorBlueprintResources/StandardMacros.DecrementInt` (`self.Playercount`))))

(fn `CheckPlayerCount`
  (if (>= (`self.Playercount`) 3)
    (`PrimitiveComponent.SetSimulatePhysics` (`self.FloorMesh`) true)
    (`self.K2_DestroyActor`)))

(fn `UserConstructionScript`)